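; Level setup Blueprint that spawns and initializes an SPH fluid Simulator on BeginPlay, configuring it by level name.
; BuildScenario creates fluids from spawners or a saved file and borders from static meshes.
; Per-level switches add border lines, periodic conditions, dimensionality, accelerations and a shear-wave sensor line.
; These feed a DFSPH solver with MLS boundary pressure, hashed neighbor search and recording through gathered cameras and sensors, alongside scripted volumes.
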(event EventBeginPlay
  (Utilities|FlowControl|Sequence
    (:then_0
      ;[1 1 1] Simulation
      (bind _returnvalue (Game|SpawnActorfromClass "/Script/Simulation.Simulator" (Math|Transform|MakeTransform "0, 0,-300.000000") "Undefined" 0 0))
      (Variables|Default|SetSimulation _returnvalue))
    (:then_1
      (CallFunction|BuildScenario))
    (:then_2
      (Utilities|FlowControl|Sequence
        (:then_0
          (bind _outactors (Actor|GetAllActorsOfClass "/Script/Simulation.ScriptedVolume"))
          (Variables|Default|SetVolumes _outactors))
        (:then_1
          (bind _outactors_2 (Actor|GetAllActorsOfClass "/Script/Simulation.RecordingCamera"))
          (Variables|Default|SetCameras _outactors_2))
        (:then_2
          (bind _outactors_3 (Actor|GetAllActorsOfClass "/Script/Simulation.Sensor"))
          (Variables|Default|SetSensors _outactors_3))))
    (:then_3
      ;[1 1 1] Build the Simulation
      (bind _returnvalue_2 (Game|GetCurrentLevelName true))
      (Class|Simulator|Initialize (Variables|Default|GetSimulation) (Class|ParticleContext|CreateParticleContext 0.2 (Variables|Default|GetFluids) (Variables|Default|GetStaticBorders) (Utilities|Struct|MakeVisualisationInformation "Velocity" true -3.0 3.0) (Variables|Default|GetPeriodicCondition)) (Class|DFSPHSolver|CreateDFSPHSolver (Variables|Default|GetAccelerations) 0.1 1.0 0.001 0.04 2 4 2 100 0.5 (Class|MLSExtrapolation|CreateBoundaryMLSExtrapolationPressureComputation (Utilities|Struct|MakeEpsilons 1e+03 1e+02 0.1)) (Class|CorrectedKernelPressureGradient|CreateCorrectedKernelPressureGradient (Utilities|Struct|MakeEpsilons 1e+03 1e+05 0.0001))) (Class|CubicSplineKernel|CreateCubicSplineKernel 2.0) (Class|HashNeighborsFinder|CreateHashNeighborsFinder) (Class|RecordManager|CreateRecordManager (Variables|Default|GetCameras) (Variables|Default|GetSensors) "Normal" "Normal" 1.2e+02 200 false) (Variables|Default|GetVolumes) 0.1 1e-05 0.001 _returnvalue_2 false (Variables|Default|GetDimensionality)))))

(fn ConstructionScript)

(fn BuildScenario
  (Utilities|FlowControl|Sequence
    (:then_0
      ;[1 1 1] Default Behavior
      (Utilities|FlowControl|Sequence
        (:then_0
          (if (Variables|Default|GetLoadFromFile)
            (bind _returnvalue (Game|GetCurrentLevelName true))
            (Utilities|Array|Add (Variables|Default|GetFluids) (Class|Fluid|CreateFluidfromFile (Utilities|String|Append (Class|Simulator|GetSimulationPath (Variables|Default|GetSimulation)) "Simulation Saves/" _returnvalue "Still" "/0.fluid")))
            (bind _outactors (Actor|GetAllActorsOfClass "/Script/Simulation.FluidSpawner"))
            (for _array_element _outactors
              (Actor|DestroyActor _array_element))
            (else
              (bind _outactors_2 (Actor|GetAllActorsOfClass "/Script/Simulation.FluidSpawner"))
              (for _array_element_2 _outactors_2
                (Utilities|Array|Add (Variables|Default|GetFluids) (Class|Fluid|CreateFluidfromSpawner _array_element_2))))))
        (:then_1
          (bind _outactors_3 (Actor|GetAllActorsOfClass "/Script/Engine.StaticMeshActor"))
          (Utilities|Array|Add (Variables|Default|GetStaticBorders) (Class|StaticBorder|CreateStaticBorderfromStaticMeshActors _outactors_3 1.0 1.0 0.9 0.04)))
        (:then_2
          (bind _outactors_4 (Actor|GetAllActorsOfClass "/Script/Simulation.Sensor"))
          (Variables|Default|SetSensors _outactors_4))))
    (:then_1
      ;[1 1 1] Static borders
      (bind _returnvalue_2 (Game|GetCurrentLevelName true))
      (switch string _returnvalue_2
        (:BreakingDam2D
          (Utilities|FlowControl|Sequence :!label _label
            (:then_0
              (Utilities|Array|Add (Variables|Default|GetStaticBorders) (Class|StaticBorder|CreateStaticBorderfromLine "-10.000000, 0,-10.000000" "10.000000, 0,-10.000000" 1.1 1.0 0.7 0.04 "0.000000,0.000000,0.000000")))
            (:then_1
              (Utilities|Array|Add (Variables|Default|GetStaticBorders) (Class|StaticBorder|CreateStaticBorderfromLine "10.000000, 0,-10.000000" "10.000000, 0,30.000000" 1.2 1.0 0.7 0.04 "0.000000,0.000000,0.000000")))
            (:then_2
              (Utilities|Array|Add (Variables|Default|GetStaticBorders) (Class|StaticBorder|CreateStaticBorderfromLine "10.000000, 0,30.000000" "-10.000000,0.000000,30.000000" 1.2 1.0 0.7 0.04 "0.000000,0.000000,0.000000")))
            (:then_3
              (Utilities|Array|Add (Variables|Default|GetStaticBorders) (Class|StaticBorder|CreateStaticBorderfromLine "-10.000000, 0,30.000000" "-10.000000, 0,-10.000000" 1.2 1.0 0.7 0.04 "0.000000,0.000000,0.000000")))))
        (:BreakingDam2DFilled
          (goto _label))
        (:PeriodicBreakingDam
          (Utilities|FlowControl|Sequence
            (:then_0
              (Utilities|Array|Add (Variables|Default|GetStaticBorders) (Class|StaticBorder|CreateStaticBorderfromLine "-20.000000, 0,9.000000" "20.000000, 0,9.000000" 1.2 1.0 0.7 0.04 "0.000000,0.000000,0.000000"))
              (Variables|Default|SetPeriodicCondition (Class|PeriodicCondition|CreatePeriodicCondition "-10.000000,-10.000000,-10.000000" "10.000000,10.000000,10.000000")))
            (:then_3
              (Utilities|Array|Add (Variables|Default|GetStaticBorders) (Class|StaticBorder|CreateStaticBorderfromLine "-20.000000, 0,8.000000" "20.000000, 0,8.000000" 1.0 1.0 0.6 0.04 "0.000000,0.000000,0.000000"))
              (Variables|Default|SetPeriodicCondition (Class|PeriodicCondition|CreatePeriodicCondition "-10.000000,-10.000000,-10.000000" "10.000000,10.000000,10.000000")))))
        (:PeriodicShearWave
          (Variables|Default|SetPeriodicCondition (Class|PeriodicCondition|CreatePeriodicCondition "-10.000000,-10.000000,-10.000000" "10.000000,10.000000,10.000000")))
        (:Empty
          (Utilities|Array|Add (Variables|Default|GetStaticBorders) (Class|StaticBorder|CreateStaticBorderfromLine "-12.000000, 0,0.000000" "-12.000000, 0,0.000000" 1.0 1.0 0.5 0.04 "0.000000,0.000000,0.000000")))))
    (:then_2
      ;[1 1 1] Dimensionality
      (bind _returnvalue_3 (Game|GetCurrentLevelName true))
      (switch string _returnvalue_3
        (:Default
          (Variables|Default|SetDimensionality "Three"))
        (:BreakingDam2D
          (Variables|Default|SetDimensionality "Two" :!label _label_2))
        (:BreakingDam2DFilled
          (goto _label_2))
        (:PeriodicBreakingDam
          (goto _label_2))
        (:PeriodicShearWave
          (goto _label_2))
        (:Empty
          (Variables|Default|SetDimensionality "One"))))
    (:then_3
      ;[1 1 1] Accelerations
      (bind _returnvalue_4 (Game|GetCurrentLevelName true))
      (switch string _returnvalue_4
        (:Default
          (Variables|Default|SetAccelerations (Utilities|Array|MakeArray (Class|Viscosity|CreateViscosity) (Class|Damping|CreateDamping 0.0) (Class|Gravity|CreateGravity "0.000000,0.000000,-9.810000") (Class|SurfaceTension|CreateSurfaceTension 0.0))))
        (:BreakingDam2D
          (Variables|Default|SetAccelerations (Utilities|Array|MakeArray (Class|Viscosity|CreateViscosity) (Class|Damping|CreateDamping 0.0) (Class|Gravity|CreateGravity "0.000000,0.000000,-9.810000") (Class|SurfaceTension|CreateSurfaceTension 0.0)) :!label _label_3))
        (:BreakingDam2DFilled
          (goto _label_3))
        (:PeriodicBreakingDam
          (goto _label_3))
        (:PeriodicShearWave
          (Variables|Default|SetAccelerations (Utilities|Array|MakeArray (Class|Viscosity|CreateViscosity))))
        (:Empty
          (Variables|Default|SetAccelerations (Utilities|Array|MakeArray (Class|Gravity|CreateGravity "-1.000000,0.000000,0.000000"))))))
    (:then_4
      ;[1 1 1] Sensors
      (bind _returnvalue_5 (Game|GetCurrentLevelName true))
      (switch string _returnvalue_5
        (:PeriodicShearWave
          (Class|LineSensor|SpawnSensorLine (Class|Simulator|GetWorldBlueprint (Variables|Default|GetSimulation)) (Utilities|Struct|MakeMeasuredAttributes false false false true false false true) "0.000000, 0,10.000000" "0, 0,-10.000000" 0.05))))))