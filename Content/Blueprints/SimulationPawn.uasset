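; Free-flying spectator pawn that serves as camera and input controller for a particle fluid simulation.
; On BeginPlay it caches the SimulationSettings game mode and adds HUD widgets; right-click toggles mouse-look, and the wheel scales flight speed.
; Input actions forward simulation, replay, visibility, volume and export commands to the game mode's Simulation subobjects.
; Debug keys take screenshots or add a particle where the camera ray hits the Y=0 plane.
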(event EventBeginPlay
  (bind _returnvalue (Game|GetPlayerController 0))
  (bind _assimulation_settings (Utilities|Casting|CastToSimulationSettings (Game|GetGameMode)))
  (Variables|Default|SetGameMode _assimulation_settings)
  (bind _returnvalue_2 (UserInterface|CreateWidget "/Game/Widget/Crossfade.Crossfade_C"))
  (UserInterface|Viewport|AddtoViewport _returnvalue_2 0)
  (bind _returnvalue_3 (UserInterface|CreateWidget "/Game/Widget/Anzeige.Anzeige_C" 0 (Variables|Default|GetGameMode)))
  (UserInterface|Viewport|AddtoViewport _returnvalue_3 0)
  (Input|SetInputModeGameandUI _returnvalue 0 "DoNotLock" false)
  (Variables|/Script/Engine.PlayerController|SetbShowMouseCursor _returnvalue true))

(event Input|ActionEvents|InputActionHideBorders
  (params (Key :type Key%20Structure))
  (bind _gamemode (Variables|Default|GetGameMode))
  (bind _simulation (Variables|/Game/Blueprints/SimulationSettings.SimulationSettings_C|GetSimulation _gamemode))
  (bind _returnvalue (Class|Simulator|GetParticleContext _simulation))
  (bind _returnvalue_2 (Class|ParticleContext|GetVisualisationInformation _returnvalue))
  (bind (_colorcode _autolimits _min _max _showfluids _showstaticborders) (Utilities|Struct|BreakVisualisationInformation _returnvalue_2))
  (:Released
    (Class|ParticleContext|SetVisualisationInformation _returnvalue (Utilities|Struct|MakeVisualisationInformation _colorcode _autolimits _min _max _showfluids (not _showstaticborders)))))

(event Input|ActionEvents|InputActionStartStopSimulation
  (params (Key :type Key%20Structure))
  (:Released
    (Class|Simulator|StartPauseSimulation (Variables|/Game/Blueprints/SimulationSettings.SimulationSettings_C|GetSimulation (Variables|Default|GetGameMode)))))

(event Input|ActionEvents|InputActionRewindToStart
  (params (Key :type Key%20Structure))
  (:Released
    (Class|RecordManager|RewindReplay (Class|Simulator|GetRecordManager (Variables|/Game/Blueprints/SimulationSettings.SimulationSettings_C|GetSimulation (Variables|Default|GetGameMode))))))

(event Input|ActionEvents|InputActionDecreaseReplaySpeed
  (params (Key :type Key%20Structure))
  (:Released
    (Class|RecordManager|DecreaseReplaySpeed (Class|Simulator|GetRecordManager (Variables|/Game/Blueprints/SimulationSettings.SimulationSettings_C|GetSimulation (Variables|Default|GetGameMode))))))

(event Input|ActionEvents|InputActionHideFluids
  (params (Key :type Key%20Structure))
  (bind _gamemode (Variables|Default|GetGameMode))
  (bind _simulation (Variables|/Game/Blueprints/SimulationSettings.SimulationSettings_C|GetSimulation _gamemode))
  (bind _returnvalue (Class|Simulator|GetParticleContext _simulation))
  (bind _returnvalue_2 (Class|ParticleContext|GetVisualisationInformation _returnvalue))
  (bind (_colorcode _autolimits _min _max _showfluids _showstaticborders) (Utilities|Struct|BreakVisualisationInformation _returnvalue_2))
  (:Released
    (Class|ParticleContext|SetVisualisationInformation _returnvalue (Utilities|Struct|MakeVisualisationInformation _colorcode _autolimits _min _max (not _showfluids) _showstaticborders))))

(event Input|ActionEvents|InputActionStartStopReplay
  (params (Key :type Key%20Structure))
  (:Released
    (Class|Simulator|StartPauseReplay (Variables|/Game/Blueprints/SimulationSettings.SimulationSettings_C|GetSimulation (Variables|Default|GetGameMode)))))

(event Input|ActionEvents|InputActionIncreaseReplaySpeed
  (params (Key :type Key%20Structure))
  (:Released
    (Class|RecordManager|IncreaseReplaySpeed (Class|Simulator|GetRecordManager (Variables|/Game/Blueprints/SimulationSettings.SimulationSettings_C|GetSimulation (Variables|Default|GetGameMode))))))

(event Input|ActionEvents|InputActionHideMeshes
  (params (Key :type Key%20Structure))
  (:Released
    (bind _outactors (Actor|GetAllActorsOfClass "/Script/Engine.StaticMeshActor"))
    (for _array_element _outactors
      (Rendering|SetActorHiddenInGame _array_element (not (Variables|/Script/Engine.Actor|GetbHidden _array_element))))))

(event Input|ActionEvents|InputActionSaveDensitiesToFile
  (params (Key :type Key%20Structure))
  (bind _gamemode (Variables|Default|GetGameMode))
  (bind _simulation (Variables|/Game/Blueprints/SimulationSettings.SimulationSettings_C|GetSimulation _gamemode))
  (bind _returnvalue (Class|Simulator|GetRecordManager _simulation))
  (:Released
    (Class|RecordManager|WriteSolverStatisticstoFile _returnvalue)
    (Class|RecordManager|WriteSensorDatatoFile _returnvalue)))

(event Input|ActionEvents|InputActionEnableVolumes
  (params (Key :type Key%20Structure))
  (:Released
    (for _array_element (Class|Solver|GetScriptedVolumes (Class|Simulator|GetSolver (Variables|/Game/Blueprints/SimulationSettings.SimulationSettings_C|GetSimulation (Variables|Default|GetGameMode))))
      (Class|ScriptedVolume|SetEnabled _array_element (not (Class|ScriptedVolume|GetEnabled _array_element))))))

(event Input|AxisEvents|InputAxisPitch
  (params (AxisValue :type Float%20%28single-precision%29))
  (bind _returnvalue (Game|GetPlayerController 0))
  (bind _returnvalue_2 (Pawn|GetControlRotation _returnvalue :!class /Script/Engine.Controller))
  (bind (_roll _pitch _yaw) (Math|Rotator|BreakRotator _returnvalue_2))
  (Pawn|SetControlRotation (Game|GetPlayerController 0) (Math|Rotator|MakeRotator _roll (Math|Float|Clamp(Float) (+ _pitch AxisValue) -85.0 85.0) _yaw)))

(event Input|AxisEvents|InputAxisForward
  (params (AxisValue :type Float%20%28single-precision%29))
  (Class|PawnMovementComponent|AddInputVector (Variables|Default|GetMovementComponent) (* (Math|Vector|GetForwardVector (Transformation|GetActorRotation)) AxisValue) false))

(event Input|AxisEvents|InputAxisYaw
  (params (AxisValue :type Float%20%28single-precision%29))
  (bind _returnvalue (Game|GetPlayerController 0))
  (bind _returnvalue_2 (Pawn|GetControlRotation _returnvalue :!class /Script/Engine.Controller))
  (bind (_roll _pitch _yaw) (Math|Rotator|BreakRotator _returnvalue_2))
  (Pawn|SetControlRotation (Game|GetPlayerController 0) (Math|Rotator|MakeRotator _roll _pitch (+ _yaw AxisValue))))

(event Input|AxisEvents|InputAxisUp
  (params (AxisValue :type Float%20%28single-precision%29))
  (Class|PawnMovementComponent|AddInputVector (Variables|Default|GetMovementComponent) (* (Math|Vector|GetUpVector (Transformation|GetActorRotation)) AxisValue) false))

(event Input|AxisEvents|InputAxisRight
  (params (AxisValue :type Float%20%28single-precision%29))
  (Class|PawnMovementComponent|AddInputVector (Variables|Default|GetMovementComponent) (* (Math|Vector|GetRightVector (Transformation|GetActorRotation)) AxisValue) false))

(event Input|KeyboardEvents|Ö
  (params (Key :type Key%20Structure))
  (bind _returnvalue (Game|GetPlayerCameraManager 0))
  (bind _returnvalue_2 (Camera|GetCameraLocation _returnvalue))
  (bind _returnvalue_3 (Camera|GetCameraRotation _returnvalue))
  (bind _returnvalue_4 (Math|Vector|GetForwardVector _returnvalue_3))
  (bind _y (Math|Vector|BreakVector _returnvalue_2))
  (bind _y_2 (Math|Vector|BreakVector _returnvalue_4))
  (bind _returnvalue_5 (/ _y _y_2))
  (bind _returnvalue_6 (* _returnvalue_5 -1.0))
  (bind _returnvalue_7 (* _returnvalue_4 _returnvalue_6))
  (bind _returnvalue_8 (+ _returnvalue_7 _returnvalue_2))
  (bind _returnvalue_9 (/ _returnvalue_8 1e+01))
  (bind (_x _y_3 _z) (Math|Vector|BreakVector _returnvalue_9))
  (:Released
    (Class|Fluid|AddParticle (Utilities|Array|Get(acopy) (Class|ParticleContext|GetFluidsBlueprint (Class|Simulator|GetParticleContext (Variables|/Game/Blueprints/SimulationSettings.SimulationSettings_C|GetSimulation (Variables|Default|GetGameMode))))) (Math|Vector|MakeVector _x 0.0 _z) "6.000000, 0, 0" false)))

(event Input|KeyboardEvents|Ü
  (params (Key :type Key%20Structure))
  (:Released
    (Class|RecordManager|TakeScreenshot (Class|Simulator|GetRecordManager (Variables|/Game/Blueprints/SimulationSettings.SimulationSettings_C|GetSimulation (Variables|Default|GetGameMode))) -1 "Screenshots")))

(event Input|MouseEvents|MouseWheelUp
  (params (Key :type Key%20Structure))
  (bind _movementcomponent (Variables|Default|GetMovementComponent))
  (:Pressed
    (bind _asfloating_pawn_movement (Utilities|Casting|CastToFloatingPawnMovement _movementcomponent))
    (Variables|/Script/Engine.FloatingPawnMovement|SetMaxSpeed _asfloating_pawn_movement (* (Class|MovementComponent|GetMaxSpeed _movementcomponent) 1.2))))

(event Input|MouseEvents|MouseWheelDown
  (params (Key :type Key%20Structure))
  (bind _movementcomponent (Variables|Default|GetMovementComponent))
  (:Pressed
    (bind _asfloating_pawn_movement (Utilities|Casting|CastToFloatingPawnMovement _movementcomponent))
    (Variables|/Script/Engine.FloatingPawnMovement|SetMaxSpeed _asfloating_pawn_movement (/ (Class|MovementComponent|GetMaxSpeed _movementcomponent) 1.2))))

(event Input|MouseEvents|RightMouseButton
  (params (Key :type Key%20Structure))
  (bind _returnvalue (Game|GetPlayerController 0))
  (bind (_locationx _locationy) (Game|Player|GetMousePosition _returnvalue))
  (:Released
    (Utilities|FlowControl|FlipFlop
      (:A
        (Input|SetInputModeGameOnly _returnvalue)
        (Variables|/Script/Engine.PlayerController|SetbShowMouseCursor _returnvalue false)
        (Variables|Default|SetMousePosition (Math|Vector2D|MakeVector2D _locationx _locationy)))
      (:B
        (Input|SetInputModeGameandUI _returnvalue 0 "DoNotLock" false)
        (Variables|/Script/Engine.PlayerController|SetbShowMouseCursor _returnvalue true)
        (Class|PlayerController|SetMouseLocation _returnvalue (Math|Float|Truncate (.X (Math|Vector2D|BreakVector2D (Variables|Default|GetMousePosition)))) (Math|Float|Truncate (.Y (Math|Vector2D|BreakVector2D (Variables|Default|GetMousePosition)))))))))

(fn ConstructionScript)